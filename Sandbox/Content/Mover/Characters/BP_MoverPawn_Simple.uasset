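; Simple test pawn for the Mover plugin that generates hardcoded input and prints movement debug info.
; ProduceInput builds character default inputs with a constant +X directional input, without reading player controls, and returns a Mover input command context.
; Tick prints the last command's move input type or a fallback message, and CharacterMover's mode-change event prints the previous and new movement modes.
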(event `self.ReceiveBeginPlay`)

(event `self.ReceiveTick`
  (params (DeltaSeconds :type "Float (single-precision)"))
  (bind (_didsucceed _targetasrawbytes) (`MoverDataCollectionLibrary.K2_GetDataFromCollection` (`.InputCollection` (break `MoverInputCmdContext` (`MoverComponent.GetLastInputCmd` (`self.CharacterMover`))))))
  (if _didsucceed
    (`KismetSystemLibrary.PrintString` (`|GetEnumeratorNameAsString` (`.MoveInputType` (break `CharacterDefaultInputs` _targetasrawbytes))))
    (else
      (`KismetSystemLibrary.PrintString` "Last Input Cmd is None."))))

(event `self.CharacterMover.OnMovementModeChanged`
  (params (PreviousMovementModeName :type "Name (by ref)") (NewMovementModeName :type "Name (by ref)"))
  (`KismetSystemLibrary.PrintText` (`|FormatText` "Mode: {0} to {1}" PreviousMovementModeName NewMovementModeName)))

(fn `ProduceInput`
  (params (SimTimeMs :type Integer))
  (returns (InputCmdResult :type "MoverInputCmdContext Structure"))
  (bind _moverdatacollection (make `MoverDataCollection`))
  (bind _characterdefaultinputs (make `CharacterDefaultInputs` (0.0 0.0 0.0)))
  (`MoverDataModelBlueprintLibrary.SetDirectionalInput` _characterdefaultinputs (`KismetMathLibrary.MakeVector` 1.0))
  (`MoverDataCollectionLibrary.K2_AddDataToCollection` _moverdatacollection _characterdefaultinputs)
  (return (make `MoverInputCmdContext` _moverdatacollection)))

(fn `UserConstructionScript`
  (`parent.UserConstructionScript`))