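; BP_MoverPlayerController is a player controller that handles basic move and look input through Enhanced Input.
; On BeginPlay it adds the IMC_Basic mapping context.
; IA_Move sends camera-relative movement input to the controlled pawn, mapping X to the camera manager's forward vector, unflattened, and Y to its right vector.
; IA_Look feeds the controller's yaw and pitch input.
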(event `self.ReceiveBeginPlay`
  (`EnhancedInputSubsystemInterface.AddMappingContext` (subsystem `EnhancedInputLocalPlayerSubsystem`) "/Game/Shared/Core/Input/IMC_Basic.IMC_Basic" 0 (struct)))

(event `EnhancedInput|/Game/Shared/Core/Input/IA_Move`
  (params (ActionValue :type "Vector2D Structure") (ElapsedSeconds :type "Float (double-precision)") (TriggeredSeconds :type "Float (double-precision)") (InputAction :type "InputAction Object Reference" :default "/Game/Shared/Core/Input/IA_Move.IA_Move"))
  (bind (_x _y) (`KismetMathLibrary.BreakVector2D` ActionValue))
  (bind _returnvalue (`GameplayStatics.GetPlayerCameraManager` 0))
  (:`Triggered`
    (`Pawn.AddMovementInput` (`self.K2_GetPawn`) (+ (* _x (`self.GetActorForwardVector` _returnvalue)) (* _y (`self.GetActorRightVector` _returnvalue))) 1.0 false)))

(event `EnhancedInput|/Game/Shared/Core/Input/IA_Look`
  (params (ActionValue :type "Vector2D Structure") (ElapsedSeconds :type "Float (double-precision)") (TriggeredSeconds :type "Float (double-precision)") (InputAction :type "InputAction Object Reference" :default "/Game/Shared/Core/Input/IA_Look.IA_Look"))
  (:`Triggered`
    (`self.AddYawInput` ActionValue_X)
    (`self.AddPitchInput` ActionValue_Y)))

(fn `UserConstructionScript`)